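; Player pawn Blueprint for an Ori-style character with side-to-side movement, jump, double jump and object dash.
; Horizontal axis input sets the Y component of Speed, while jump input picks normal or double jump, stopping normal jumps on release or after a delay.
; ObjectDashScope overlaps maintain the Objects list, from which dash input selects a target and dashes along a fixed direction unless sky-dashing.
; Debug prints remain on overlap and dash.
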(event Custom|OnComponentBeginOverlap_Event_0
  (params (OverlappedComponent :type Primitive%20Component%20Object%20Reference) (OtherActor :type Actor%20Object%20Reference) (OtherComp :type Primitive%20Component%20Object%20Reference) (OtherBodyIndex :type Integer) (bFromSweep :type Boolean) (SweepResult :type Hit%20Result%20Structure%20%28by%20ref%29))
  (Utilities|Array|AddUnique (Variables|Default|Getobjects) OtherActor)
  (Development|PrintString "Hello"))

(event Custom|OnComponentEndOverlap_Event_0
  (params (OverlappedComponent :type Primitive%20Component%20Object%20Reference) (OtherActor :type Actor%20Object%20Reference) (OtherComp :type Primitive%20Component%20Object%20Reference) (OtherBodyIndex :type Integer))
  (Utilities|Array|RemoveItem (Variables|Default|Getobjects) OtherActor))

(event EventBeginPlay
  (bind _objectdashscope (Variables|Default|GetObjectDashScope))
  (|CallParentFunction)
  (Collision|AssignOnComponentBeginOverlap _objectdashscope (delegate Custom|OnComponentBeginOverlap_Event_0))
  (Collision|AssignOnComponentEndOverlap _objectdashscope (delegate Custom|OnComponentEndOverlap_Event_0))
  (Variables|Default|Setobjects (Collision|GetOverlappingActors (Variables|Default|GetObjectDashScope) "/Script/Engine.Actor" :!class /Script/Engine.PrimitiveComponent)))

(event Collision|EventActorBeginOverlap
  (params (OtherActor :type Actor%20Object%20Reference)))

(event EventTick
  (params (DeltaSeconds :type Float%20%28single-precision%29)))

(event Input|ActionEvents|InputActionJump
  (params (Key :type Key%20Structure :default "None"))
  (:Pressed
    (if (Variables|Default|GetisJump)
      (if (not (Variables|Default|GetisDoubleJump))
        (Class|OriPawn|DoubleJump))
      (else
        (Class|OriPawn|NormalJump)
        (Utilities|FlowControl|Delay 0.7)
        (Class|OriPawn|NormalJumpStop))))
  (:Released
    (Class|OriPawn|NormalJumpStop)))

(event Input|ActionEvents|InputActionObjectDash
  (params (Key :type Key%20Structure :default "None"))
  (bind _objects (Variables|Default|Getobjects))
  (:Pressed
    (if (not (Variables|Default|GetisSkyDash))
      (bind _returnvalue (Class|OriPawn|ObjectDashBegin _objects))
      (Development|PrintString (Utilities|String|ToString(Integer) (Utilities|Array|Length _objects)))
      (Utilities|IsValid _returnvalue
        (:Is%20Valid
          (Class|OriPawn|ObjectDash "0.000000,1.000000, 0"))))))

(event Input|AxisEvents|InputAxisMoveRight
  (params (AxisValue :type Float%20%28single-precision%29))
  (Variables|Default|SetSpeed (Math|Vector|MakeVector (.x (Variables|Default|GetSpeed)) (* AxisValue (* (Variables|Default|GetMoveSpeed) -1.0)) (.z (Variables|Default|GetSpeed)))))

(fn ConstructionScript)